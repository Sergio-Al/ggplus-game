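; BP_TileActor is a track tile that chains endless-runner style level generation as the player moves through it.
; When ThirdPersonCharacter overlaps its TileGenerator component, it asks ThirdPersonGameMode to spawn another tile, then destroys itself after a short delay.
; SpawnObstacle randomly either spawns a BP_Block1 at the Left component or spawns nothing, but its call in the event graph is unconnected and never runs.
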(event `self.ReceiveBeginPlay`)

(event `self.TileGenerator.OnComponentBeginOverlap`
  (params (OverlappedComponent :type "PrimitiveComponent Object Reference") (OtherActor :type "Actor Object Reference") (OtherComp :type "PrimitiveComponent Object Reference") (OtherBodyIndex :type Integer) (bFromSweep :type Boolean) (SweepResult :type "HitResult Structure (by ref)"))
  (cast `/Game/ThirdPersonBP/Blueprints/ThirdPersonCharacter` OtherActor)
  (bind _asthird_person_game_mode (cast `/Game/ThirdPersonBP/Blueprints/ThirdPersonGameMode` (`GameplayStatics.GetGameMode`)))
  (`/Game/ThirdPersonBP/Blueprints/ThirdPersonGameMode.SpawnTile` _asthird_person_game_mode)
  (`KismetSystemLibrary.Delay` 0.5)
  (`self.K2_DestroyActor`))

(fn `SpawnObstacle`
  (switch `int` (`KismetMathLibrary.RandomIntegerInRange` 0 1)
    (:`1`
      (`|SpawnActorFromClass` "/Game/Gameplay/Blueprint/BP_Block1.BP_Block1_C" (`SceneComponent.K2_GetComponentToWorld` (`self.Left`)) "Undefined" "OverrideRootScale" null null))))

(fn `UserConstructionScript`)