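; BP_Block1 is a short-lived hazard block that damages the ThirdPersonCharacter when the two collide.
; A hit on its Cube component by that character spawns a blood particle effect, sets the cube to ignore Pawn collision, applies fixed damage and destroys the block.
; Independently, a delay started on BeginPlay destroys the block after a few seconds.
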(event `self.ReceiveBeginPlay`
  (`KismetSystemLibrary.Delay` 5.0)
  (`self.K2_DestroyActor`))

(event `self.Cube.OnComponentHit`
  (params (HitComponent :type "PrimitiveComponent Object Reference") (OtherActor :type "Actor Object Reference") (OtherComp :type "PrimitiveComponent Object Reference") (NormalImpulse :type "Vector Structure") (Hit :type "HitResult Structure (by ref)"))
  (bind _asthird_person_character (cast `/Game/ThirdPersonBP/Blueprints/ThirdPersonCharacter` OtherActor))
  (`GameplayStatics.SpawnEmitterAtLocation` "/Game/FXVarietyPack/Particles/P_Blood.P_Blood" (`SceneComponent.K2_GetComponentLocation` (`self.Cube`)))
  (`PrimitiveComponent.SetCollisionResponseToChannel` (`self.Cube`) "ECC_Pawn" "ECR_Ignore")
  (`GameplayStatics.ApplyDamage` _asthird_person_character 10.0)
  (`self.K2_DestroyActor`))

(fn `UserConstructionScript`)