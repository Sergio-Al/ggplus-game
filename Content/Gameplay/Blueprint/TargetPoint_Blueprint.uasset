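; Obstacle spawner that follows the first BPC_EnemyBase actor found at BeginPlay, held 500 units from it on negative X every Tick.
; A BeginPlay delay loop calls SpawnObstacles every three seconds to pick one of three target points at random.
; SpawnActorAtLocation plays a thunder-ball hit effect there and spawns a random class from BlockPositions, or prints a warning if that array is empty.
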(event `self.ReceiveBeginPlay`
  (bind _returnvalue (`GameplayStatics.GetActorOfClass` "/Game/Character/NPC/BPC_EnemyBase.BPC_EnemyBase_C"))
  (set `self.EnemyActor` _returnvalue)
  (`self.SpawnObstacles` :!label _label)
  (`KismetSystemLibrary.Delay` 3.0)
  (goto _label))

(event `self.ReceiveTick`
  (params (DeltaSeconds :type "Float (single-precision)"))
  (bind (_returnvalue_x _returnvalue_y _returnvalue_z) (`KismetMathLibrary.BreakVector` (`self.K2_GetActorLocation` (`self.EnemyActor`))))
  (`self.K2_SetActorLocation` (`KismetMathLibrary.MakeVector` (- _returnvalue_x 500.0) _returnvalue_y _returnvalue_z)))

(fn `SpawnActorAtLocation`
  (params (Location :type "Vector Structure") (Rotation :type "Rotator Structure"))
  (bind _returnvalue (`KismetMathLibrary.MakeTransform` Location Rotation))
  (bind _blockpositions (`self.BlockPositions`))
  (if (> (`KismetArrayLibrary.Array_Length` _blockpositions) 0)
    (`GameplayStatics.SpawnEmitterAtLocation` "/Game/FXVarietyPack/Particles/P_ky_ThunderBallHit.P_ky_ThunderBallHit" (.location _returnvalue) (.rotation _returnvalue) (.scale _returnvalue))
    (`|SpawnActorFromClass` (`|GetArrayItem` _blockpositions (`KismetMathLibrary.RandomIntegerInRange` 0 (`KismetArrayLibrary.Array_LastIndex` _blockpositions))) _returnvalue "AlwaysSpawn" "OverrideRootScale" null null)
    (else
      (`KismetSystemLibrary.PrintString` "your class is empty"))))

(fn `SpawnObstacles`
  (switch `int` (`KismetMathLibrary.RandomIntegerInRange` 0 2)
    (:`0`
      (`self.SpawnActorAtLocation` (.location (`SceneComponent.K2_GetComponentToWorld` (`self.TargetPoint_1`))) (.rotation (`SceneComponent.K2_GetComponentToWorld` (`self.TargetPoint_1`)))))
    (:`1`
      (`self.SpawnActorAtLocation` (.location (`SceneComponent.K2_GetComponentToWorld` (`self.TargetPoint_2`))) (.rotation (`SceneComponent.K2_GetComponentToWorld` (`self.TargetPoint_2`)))))
    (:`2`
      (`self.SpawnActorAtLocation` (.location (`SceneComponent.K2_GetComponentToWorld` (`self.TargetPoint_3`))) (.rotation (`SceneComponent.K2_GetComponentToWorld` (`self.TargetPoint_3`)))))))

(fn `UserConstructionScript`)