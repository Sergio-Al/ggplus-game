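; BP_MinionCharacter is a minion NPC character that constantly moves forward and attacks the player's ThirdPersonCharacter.
; Each Tick it forces movement input along its control yaw, with pitch and roll zeroed to stay on the plane.
; Overlapping the AttackEnemy component plays a sped-up attack montage.
; Damage is applied separately, when the player leaves the Sphere component's overlap, rather than from the montage.
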(event `self.ReceiveBeginPlay`)

(event `self.ReceiveTick`
  (params (DeltaSeconds :type "Float (single-precision)"))
  (`self.AddMovementInput` (`KismetMathLibrary.GetForwardVector` (`KismetMathLibrary.MakeRotator` 0.0 0.0 (.yaw (`self.GetControlRotation`)))) 1.0 true))

(event `self.AttackEnemy.OnComponentBeginOverlap`
  (params (OverlappedComponent :type "PrimitiveComponent Object Reference") (OtherActor :type "Actor Object Reference") (OtherComp :type "PrimitiveComponent Object Reference") (OtherBodyIndex :type Integer) (bFromSweep :type Boolean) (SweepResult :type "HitResult Structure (by ref)"))
  (cast `/Game/ThirdPersonBP/Blueprints/ThirdPersonCharacter` OtherActor)
  (`self.PlayAnimMontage` "/Game/Character/NPC/Minion/Animations/AM_MinionAttack.AM_MinionAttack" 1.25))

(event `self.Sphere.OnComponentEndOverlap`
  (params (OverlappedComponent :type "PrimitiveComponent Object Reference") (OtherActor :type "Actor Object Reference") (OtherComp :type "PrimitiveComponent Object Reference") (OtherBodyIndex :type Integer))
  (bind _asthird_person_character (cast `/Game/ThirdPersonBP/Blueprints/ThirdPersonCharacter` OtherActor))
  (`GameplayStatics.ApplyDamage` _asthird_person_character 20.0))

(fn `UserConstructionScript`)